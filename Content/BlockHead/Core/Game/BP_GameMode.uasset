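; BlockHead game mode that sets up the player's HUD and input when play begins.
; On BeginPlay it creates and stores a WBP_HUD widget, adds it to the viewport, then hides the mouse cursor and switches to game-only input.
; End game, level complete, next level, restart and game complete functions are placeholders that only print debug strings.
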(event EventBeginPlay
  (bind _returnvalue (Game|GetPlayerController 0))
  ;[0.1062 1 0.2026] Begin Play Sequence
  (Utilities|FlowControl|Sequence
    (:then_0
      ;[0.1062 1 0.2026] Add HUD to Viewport
      (bind _returnvalue_2 (UserInterface|CreateWidget "/Game/BlockHead/Core/UI/WBP_HUD.WBP_HUD_C"))
      (Variables|Default|SetHUD _returnvalue_2)
      (UserInterface|Viewport|AddtoViewport (Variables|Default|GetHUD) 0))
    (:then_1
      ;[0.1062 1 0.2026] Hide Mouse Pointer and Set Input Mode to Game Only (Capture Keyboard Input Automatically)
      (Variables|/Script/Engine.PlayerController|SetbShowMouseCursor _returnvalue false)
      (Input|SetInputModeGameOnly _returnvalue false))))

(fn ConstructionScript)

(fn EndGame
  (Development|PrintString "End Game"))

(fn LevelComplete
  (Development|PrintString "Level Complete"))

(fn LoadNextLevel
  (Development|PrintString "Load Next Level"))

(fn RestartGame
  (Development|PrintString "Restart Game"))

(fn GameComplete
  (Development|PrintString "Game Complete"))